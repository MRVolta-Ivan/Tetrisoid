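; Tetris-style block actor made of four mesh cells, cached in an array and scaled down at BeginPlay.
; BlockRotation cycles through 90-degree pitch steps up to RotMax, then reverts using the RotRestore lookup if the new pose collides.
; DetectCollision box-traces each cell on the Visibility channel, in place for rotation or one grid step away for down, left or right, and reports the first hit.
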(event Custom|BlockRotation
  ;[1 1 1] Проверяем можем ли сделать поворот, если можем то поворачиваемся
  (if (> (Variables|Default|GetRotMax) 0)
    (bind _output_get (Variables|Default|SetRot (+ (Variables|Default|GetRot) 1)))
    (if (> _output_get (Variables|Default|GetRotMax))
      (Variables|Default|SetRot 0))
    (Transformation|SetActorRotation (Math|Rotator|MakeRotator 0.0 (Math|Conversions|ToFloat(Integer) (* (Variables|Default|GetRot) 90)) 0.0))
    (bind _iscollision (CallFunction|DetectCollision true false false))
    (if _iscollision
      (Transformation|SetActorRotation (Math|Rotator|MakeRotator 0.0 (Math|Conversions|ToFloat(Integer) (Utilities|Array|Get(acopy) (Variables|Default|GetRotRestore) (Variables|Default|GetRot))) 0.0))
      (Variables|Default|SetRot (- (Variables|Default|GetRot) 1)))))

(event EventBeginPlay
  (bind _returnvalue (Transformation|GetActorTransform))
  ;[1 1 1] Сохраняем 4 блока в массиве
  (Variables|Default|SetAllBlock (Utilities|Array|MakeArray (Variables|Default|GetSM_Center) (Variables|Default|GetSM_01) (Variables|Default|GetSM_02) (Variables|Default|GetSM_03)))
  (Transformation|SetActorTransform (Math|Transform|MakeTransform (.location _returnvalue) "0, 0, 0" (/ (.scale _returnvalue) 2.56))))

(fn ConstructionScript)

(fn DetectCollision
  (params (Rot :type Boolean) (Down :type Boolean) (Left :type Boolean))
  ;[1 1 1] Проверяет нахождения припяствия по определённому действию
  (if Rot
    (LocalVariables|SetL_Location "0, 0, 0")
    (elif Down
      (LocalVariables|SetL_Location "0, 0,100.000000")
      (elif Left
        (LocalVariables|SetL_Location "100.000000, 0, 0")
        (else
          (LocalVariables|SetL_Location "-100.000000, 0, 0")))))
  (bind _array_element (Utilities|Array|ForEachLoopwithBreak (Variables|Default|GetAllBlock) :!label _label)
    (:LoopBody
      (bind _returnvalue (Collision|BoxTraceByChannel (- (Transformation|GetWorldLocation _array_element) (LocalVariables|GetL_Location)) (+ (- (Transformation|GetWorldLocation _array_element) (LocalVariables|GetL_Location)) "0,40.000000, 0") "45.000000,20.000000,45.000000" "0, 0, 0" "TraceTypeQuery1" false 0 "None"))
      (if _returnvalue
        (goto _label Break)))
    (:Completed
      (return _returnvalue))))