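; Static block for the Tetrisoid game that takes damage from ball hits and carries a score value.
; On BeginPlay, blocks with Abilities get a higher score and a glow effect, made by a timeline whose truncated track value selects among five color materials.
; DamageAndDestroy lowers Durability, or on the last hit destroys the actor with a sound, and returns whether the block was destroyed.
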(event EventBeginPlay
  ;[1 1 1] При появлении добавляет анимацию свечения блоку
  (if (> (Variables|Default|GetAbilities) 0)
    (Variables|Default|SetScore 1500)
    (bind _newtrack_0 (Timeline|Animation Play)
      (:Update
        (Rendering|Material|SetMaterial (Variables|Default|GetStaticMesh) 0 (Utilities|Select :Index (Math|Float|Truncate _newtrack_0) :Option%200 "/Game/Material/Mi_Color_08.Mi_Color_08" :Option%201 "/Game/Material/Mi_Color_09.Mi_Color_09" :Option%202 "/Game/Material/Mi_Color_10.Mi_Color_10" :Option%203 "/Game/Material/Mi_Color_11.Mi_Color_11" :Option%204 "/Game/Material/Mi_Color_12.Mi_Color_12"))))
    (else
      (Variables|Default|SetScore 300))))

(fn ConstructionScript)

(fn DamageandDestroy
  ;[1 1 1] Разрушения блока при попадании в него мячика
  (if (> (Variables|Default|GetDurability) 1)
    (Variables|Default|SetDurability (- (Variables|Default|GetDurability) 1))
    (return false)
    (else
      (Actor|DestroyActor)
      (Audio|PlaySoundatLocation "/Game/Sound/Hit3_Cue.Hit3_Cue" "0, 0, 0" "0, 0, 0" 2.0 1.0 0.0 0 0 0)
      (return true))))