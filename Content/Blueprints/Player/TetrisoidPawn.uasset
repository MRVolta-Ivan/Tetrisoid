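; Player pawn for the Tetrisoid game that relays player input to the Bp_Tetrisoid actor.
; On BeginPlay it caches the first Bp_Tetrisoid found in the level.
; Left, Right, Down and Turn input actions pass pressed and released states as booleans to its key functions, with Turn mapped to KeyUp.
; The Pause action calls PauseGame on press only, and the pawn holds no game logic itself.
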(event EventBeginPlay
  ;[1 1 1] Создаём tetrisoid
  (bind _outactors (Actor|GetAllActorsOfClass "/Game/Blueprints/Tetrisoid/Bp_Tetrisoid.Bp_Tetrisoid_C"))
  (Variables|Default|SetRef_Tetrisoid (Utilities|Array|Get(acopy) _outactors)))

(event Input|ActionEvents|InputActionLeft
  (params (Key :type Key%20Structure :default "None"))
  (bind _ref_tetrisoid (Variables|Default|GetRef_Tetrisoid))
  ;[1 1 1] Вызывает события на кнопки управления
  (:Pressed
    (Default|KeyLeft _ref_tetrisoid true))
  (:Released
    (Default|KeyLeft _ref_tetrisoid false)))

(event Input|ActionEvents|InputActionRight
  (params (Key :type Key%20Structure :default "None"))
  (bind _ref_tetrisoid (Variables|Default|GetRef_Tetrisoid))
  ;[1 1 1] Вызывает события на кнопки управления
  (:Pressed
    (Default|KeyRight _ref_tetrisoid true))
  (:Released
    (Default|KeyRight _ref_tetrisoid false)))

(event Input|ActionEvents|InputActionTurn
  (params (Key :type Key%20Structure :default "None"))
  (bind _ref_tetrisoid (Variables|Default|GetRef_Tetrisoid))
  ;[1 1 1] Вызывает события на кнопки управления
  (:Pressed
    (Default|KeyUp _ref_tetrisoid true))
  (:Released
    (Default|KeyUp _ref_tetrisoid false)))

(event Input|ActionEvents|InputActionDown
  (params (Key :type Key%20Structure :default "None"))
  (bind _ref_tetrisoid (Variables|Default|GetRef_Tetrisoid))
  ;[1 1 1] Вызывает события на кнопки управления
  (:Pressed
    (Default|KeyDown _ref_tetrisoid true))
  (:Released
    (Default|KeyDown _ref_tetrisoid false)))

(event Input|ActionEvents|InputActionPause
  (params (Key :type Key%20Structure :default "None"))
  ;[1 1 1] Вызывает события на кнопки управления
  (:Pressed
    (Default|PauseGame (Variables|Default|GetRef_Tetrisoid))))

(fn ConstructionScript)